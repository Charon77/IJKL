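; Player-controlled ship that rotates and translates using its PhysicsThrusterComponents.
; Input axes form a vector, projected onto each thruster's torque axis (location cross direction) or thrust direction to set strength.
; Positively contributing thrusters fire and spawn flame emitters.
; Tick prints thruster directions, steers a roll-free spring arm, and calls StopAllThrusters, which returns after zeroing the first thruster.
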(event `InputAxis|Rotate Pitch`
  (params (AxisValue :type "Float (single-precision)"))
  (bind _returnvalue (`KismetMathLibrary.MakeVector` (stale `InputAxis|Rotate Roll` AxisValue) AxisValue (stale `InputAxis|Rotate Yaw` AxisValue)))
  (`/Engine/EditorBlueprintResources/StandardMacros.CompareFloat` (`KismetMathLibrary.VSize` _returnvalue) :!label _label ; Prevent divide by 0
    (:`>`
      _)
    (:`<`
      _))
  (for _array_element (`self.K2_GetComponentsByClass` "/Script/Engine.PhysicsThrusterComponent")
    (bind _returnvalue_2 (`KismetMathLibrary.Normal` _returnvalue))
    (bind _returnvalue_3 (* (`KismetMathLibrary.Dot_VectorVector` (`KismetMathLibrary.ProjectVectorOnToVector` (`KismetMathLibrary.Normal` (`KismetMathLibrary.Cross_VectorVector` (`SceneComponent.RelativeLocation` _array_element) (`KismetMathLibrary.Conv_RotatorToVector` (`SceneComponent.RelativeRotation` _array_element)))) _returnvalue_2) _returnvalue_2) (`self.ThrustStrength`)))
    (`/Engine/EditorBlueprintResources/StandardMacros.CompareFloat` _returnvalue_3
      (:`>`
        (set `PhysicsThrusterComponent.ThrustStrength` _returnvalue_3 _array_element)
        (`GameplayStatics.SpawnEmitterAtLocation` "/Game/Blueprints/Flame.Flame" (`SceneComponent.K2_GetComponentLocation` _array_element) (`SceneComponent.K2_GetComponentRotation` _array_element))))))

(event `InputAxis|Rotate Roll`
  (params (AxisValue :type "Float (single-precision)"))
  (goto _label))

(event `InputAxis|Rotate Yaw`
  (params (AxisValue :type "Float (single-precision)"))
  (goto _label))

(event `self.ReceiveTick`
  (params (DeltaSeconds :type "Float (single-precision)"))
  (bind _springarm (`self.SpringArm`))
  (bind (_yaw _pitch) (`KismetMathLibrary.GetYawPitchFromVector` (`KismetMathLibrary.Conv_RotatorToVector` (`SceneComponent.RelativeRotation` _springarm))))
  (for _array_element (`self.K2_GetComponentsByClass` "/Script/Engine.PhysicsThrusterComponent")
    (`KismetSystemLibrary.PrintText` (`KismetTextLibrary.Conv_StringToText` (`KismetStringLibrary.Conv_VectorToString` (`KismetMathLibrary.Conv_RotatorToVector` (`KismetMathLibrary.NormalizedDeltaRotator` (`SceneComponent.K2_GetComponentRotation` _array_element) (`SceneComponent.K2_GetComponentRotation` (`self.K2_GetRootComponent`))))))))
  (`SceneComponent.K2_SetRelativeRotation` _springarm (`KismetMathLibrary.MakeRotator` 0.0 _pitch _yaw) false false)
  (`SceneComponent.K2_AddRelativeRotation` _springarm (`KismetMathLibrary.MakeRotator` 0.0 (`self.GetInputAxisKeyValue`) (`self.GetInputAxisKeyValue`)) false false)
  (`self.StopAllThrusters`))

(event `InputAxis|Translate Forward`
  (params (AxisValue :type "Float (single-precision)"))
  (bind _returnvalue (`KismetMathLibrary.MakeVector` AxisValue (stale `InputAxis|Translate Right` AxisValue) (stale `InputAxis|Translate Up` AxisValue)))
  (`/Engine/EditorBlueprintResources/StandardMacros.CompareFloat` (`KismetMathLibrary.VSize` _returnvalue) :!label _label_2
    (:`>`
      (for _array_element (`self.K2_GetComponentsByClass` "/Script/Engine.PhysicsThrusterComponent")
        (bind _returnvalue_2 (* (`KismetMathLibrary.Dot_VectorVector` (`KismetMathLibrary.ProjectVectorOnToVector` (`KismetMathLibrary.Conv_RotatorToVector` (`SceneComponent.RelativeRotation` _array_element)) _returnvalue) _returnvalue) (`self.ThrustStrength`)))
        (`/Engine/EditorBlueprintResources/StandardMacros.CompareFloat` _returnvalue_2
          (:`>`
            (set `PhysicsThrusterComponent.ThrustStrength` _returnvalue_2 _array_element)
            (`GameplayStatics.SpawnEmitterAtLocation` "/Game/Blueprints/Flame.Flame" (`SceneComponent.K2_GetComponentLocation` _array_element) (`SceneComponent.K2_GetComponentRotation` _array_element))))))))

(event `InputAxis|Translate Right`
  (params (AxisValue :type "Float (single-precision)"))
  (goto _label_2))

(event `InputAxis|Translate Up`
  (params (AxisValue :type "Float (single-precision)"))
  (goto _label_2))

(fn `UserConstructionScript`)